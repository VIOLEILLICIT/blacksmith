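; BP_Old_tree is an interactable tree that gives the player one item from its item data asset.
; Box overlap with the third-person character sets an in-range flag and shows or hides the interaction widget, labeled "장수 나무" on BeginPlay.
; The actor enables its own input, so IA_Interactive, while in range, prints a logging message and adds the item to the player's inventory.
; The tree itself is never removed or depleted.
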(event `self.Box.OnComponentBeginOverlap`
  (params (OverlappedComponent :type "PrimitiveComponent Object Reference") (OtherActor :type "Actor Object Reference") (OtherComp :type "PrimitiveComponent Object Reference") (OtherBodyIndex :type Integer) (bFromSweep :type Boolean) (SweepResult :type "HitResult Structure (by ref)"))
  (cast `/Game/ThirdPerson/Blueprints/BP_ThirdPersonCharacter` OtherActor)
  (set `self.PlayerInRange` true)
  (`SceneComponent.SetVisibility` (`self.interactionUI`) true false))

(event `self.Box.OnComponentEndOverlap`
  (params (OverlappedComponent :type "PrimitiveComponent Object Reference") (OtherActor :type "Actor Object Reference") (OtherComp :type "PrimitiveComponent Object Reference") (OtherBodyIndex :type Integer))
  (cast `/Game/ThirdPerson/Blueprints/BP_ThirdPersonCharacter` OtherActor)
  (set `self.PlayerInRange` false)
  (`SceneComponent.SetVisibility` (`self.interactionUI`) false false))

(event `EnhancedInput|/Game/ThirdPerson/Input/Actions/IA_Interactive`
  (params (ActionValue :type "Float (double-precision)") (ElapsedSeconds :type "Float (double-precision)") (TriggeredSeconds :type "Float (double-precision)") (InputAction :type "InputAction Object Reference" :default "/Game/ThirdPerson/Input/Actions/IA_Interactive.IA_Interactive"))
  (:`Started`
    (if (`self.PlayerInRange`)
      (`KismetSystemLibrary.PrintString` "앙 벌목띄")
      (bind _asbp_third_person_character (cast `/Game/ThirdPerson/Blueprints/BP_ThirdPersonCharacter` (`GameplayStatics.GetPlayerCharacter` 0)))
      (`InventoryComponent.AddItem` (`/Game/ThirdPerson/Blueprints/BP_ThirdPersonCharacter.Inventory` _asbp_third_person_character) (`self.item_data_asset`) 1))))

(event `self.ReceiveBeginPlay`
  (bind _interactionui (`self.interactionUI`))
  (bind _aswbp_button_ingame (cast `/Game/WBP/WBP_ButtonIngame` (`WidgetComponent.GetUserWidgetObject` _interactionui)))
  (set `/Game/WBP/WBP_ButtonIngame.AreaName` "장수 나무" _aswbp_button_ingame)
  (`SceneComponent.SetVisibility` _interactionui false false)
  (`self.EnableInput` (`GameplayStatics.GetPlayerController` 0)))

(fn `UserConstructionScript`)