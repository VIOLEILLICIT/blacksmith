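; BP_Bed is an interactable bed that lets the player sleep to advance to the next day.
; On Interact, it asks BP_GameMode1 whether the bed can be used.
; If allowed, it fades the camera out, calls SleepAndNextDay on the game mode, then fades back in.
; Otherwise, it opens a WBP_talk widget, gives it keyboard focus after a short delay, and shows the game mode's denial message.
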(event `self.Interact`
  (params (Interactor :type "Actor Object Reference"))
  (bind _asbp_game_mode_1 (cast `/Game/jungbum/BP_GameMode1` (`GameplayStatics.GetGameMode`)))
  (bind (_outdenymessage _returnvalue) (`BlacksmithGameMode.CheckCanUseBed` _asbp_game_mode_1))
  (if _returnvalue
    (`PlayerCameraManager.StartCameraFade` :`self` (`GameplayStatics.GetPlayerCameraManager` 0) :`ToAlpha` 1.0 :`Duration` 1.5 :`bHoldWhenFinished` true)
    (`KismetSystemLibrary.Delay` 1.5)
    (bind _asbp_game_mode_1_2 (cast `/Game/jungbum/BP_GameMode1` (`GameplayStatics.GetGameMode`)))
    (`BlacksmithGameMode.SleepAndNextDay` _asbp_game_mode_1_2)
    (`PlayerCameraManager.StartCameraFade` :`self` (`GameplayStatics.GetPlayerCameraManager` 0) :`FromAlpha` 1.0 :`Duration` 1.5)
    (else
      (bind _returnvalue_2 (`|CreateWidget` "/Game/jungbum/object/WBP_talk.WBP_talk_C"))
      (`UserWidget.AddToViewport` _returnvalue_2 0)
      (`KismetSystemLibrary.Delay` 0.2)
      (`Widget.SetKeyboardFocus` _returnvalue_2)
      (`/Game/jungbum/object/WBP_talk.Show Deny Message` _returnvalue_2 _outdenymessage))))

(fn `UserConstructionScript`)