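; BP_RegionZone is a placeable trigger zone that tells BP_RegionManager when the player is in its region.
; On overlap by BP_ThirdPersonCharacter, it finds the manager and calls ChangeRegion with its region ID, display name, BGM and enter sound.
; After a short delay at BeginPlay, it makes the same call if the player already starts inside the trigger, though without the manager validity check.
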(event `self.ReceiveBeginPlay`
  (`KismetSystemLibrary.Delay` 0.2)
  (if (`PrimitiveComponent.IsOverlappingActor` (`self.RegionTrigger`) (`GameplayStatics.GetPlayerCharacter` 0))
    (bind _returnvalue (`GameplayStatics.GetActorOfClass` "/Game/Jinuk/BP_RegionManager.BP_RegionManager_C"))
    (`/Game/Jinuk/BP_RegionManager.ChangeRegion` _returnvalue (`self.RegionID`) (`self.DisplayName`) (`self.RegionBGM`) (`self.EnterSFX `))))

(event `self.RegionTrigger.OnComponentBeginOverlap`
  (params (OverlappedComponent :type "PrimitiveComponent Object Reference") (OtherActor :type "Actor Object Reference") (OtherComp :type "PrimitiveComponent Object Reference") (OtherBodyIndex :type Integer) (bFromSweep :type Boolean) (SweepResult :type "HitResult Structure (by ref)"))
  (cast `/Game/ThirdPerson/Blueprints/BP_ThirdPersonCharacter` OtherActor)
  (bind _returnvalue (`GameplayStatics.GetActorOfClass` "/Game/Jinuk/BP_RegionManager.BP_RegionManager_C"))
  (`/Engine/EditorBlueprintResources/StandardMacros.IsValid` _returnvalue
    (:`Is Valid`
      (`/Game/Jinuk/BP_RegionManager.ChangeRegion` _returnvalue (`self.RegionID`) (`self.DisplayName`) (`self.RegionBGM`) (`self.EnterSFX `)))))

(fn `UserConstructionScript`)