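; BP_BattleDarkZone is a box trigger volume that switches the player's battle spotlight on inside a dark battle area and off outside it.
; After a short BeginPlay delay it caches the player as BP_ThirdPersonCharacter, then polls the box overlap on a looping timer instead of using overlap events or Tick.
; A PlayerInside flag ensures EnableBattleSpotLight and DisableBattleSpotLight are called only when the player's state changes.
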(event `self.ReceiveBeginPlay`
  (`KismetSystemLibrary.Delay` 0.2)
  (bind _asbp_third_person_character (cast `/Game/ThirdPerson/Blueprints/BP_ThirdPersonCharacter` (`GameplayStatics.GetPlayerCharacter` 0)))
  (set `self.PlayerRef` _asbp_third_person_character)
  (`self.CheckBattleZone`)
  (`KismetSystemLibrary.K2_SetTimerDelegate` (delegate `CheckBattleZone`) 0.2 true))

(event `self.ReceiveActorBeginOverlap`
  (params (OtherActor :type "Actor Object Reference")))

(event `CheckBattleZone`
  (bind _playerref (`self.PlayerRef`))
  (if (`PrimitiveComponent.IsOverlappingActor` (`self.Box`) _playerref)
    (if (not (`self.bPlayerInside`))
      (set `self.bPlayerInside` true)
      (`/Game/ThirdPerson/Blueprints/BP_ThirdPersonCharacter.EnableBattleSpotLight` _playerref))
    (elif (`self.bPlayerInside`)
      (set `self.bPlayerInside` false)
      (`/Game/ThirdPerson/Blueprints/BP_ThirdPersonCharacter.DisableBattleSpotLight` _playerref))))

(fn `UserConstructionScript`)