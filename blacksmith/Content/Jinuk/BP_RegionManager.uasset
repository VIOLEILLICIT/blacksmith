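; Region manager actor that handles the player-facing feedback when the current region changes: name display, sound effect and background music.
; BeginPlay creates the WBP_RegionName widget and adds it to the viewport.
; ChangeRegion ignores a repeated region ID, otherwise shows the name, plays the SFX and crossfades to a different BGM track.
; The music switch runs only when both the widget and the new SFX are valid.
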(event `self.ReceiveBeginPlay`
  (bind _returnvalue (`|CreateWidget` "/Game/Jinuk/WBP_RegionName.WBP_RegionName_C" (`GameplayStatics.GetPlayerController` 0)))
  (`UserWidget.AddToViewport` _returnvalue 0)
  (set `self.RegionWidget` _returnvalue))

(fn `ChangeRegion`
  (params (NewRegionID :type Name) (NewDisplayName :type Text) (NewBGM :type "SoundBase Object Reference") (NewSFX :type "SoundBase Object Reference"))
  (bind _regionwidget (`self.RegionWidget`))
  (bind _currentbgmcomponent (`self.CurrentBGMComponent`))
  (bind _fadetime (`self.FadeTime`))
  (if (== (`self.CurrentRegionID`) NewRegionID)
    (return)
    (else
      (set `self.CurrentRegionID` NewRegionID)
      (`/Engine/EditorBlueprintResources/StandardMacros.IsValid` _regionwidget
        (:`Is Valid`
          (`/Game/Jinuk/WBP_RegionName.ShowRegionName` _regionwidget NewDisplayName)
          (`KismetSystemLibrary.PrintString` "ShowRegionName 실행됨")
          (`/Engine/EditorBlueprintResources/StandardMacros.IsValid` NewSFX
            (:`Is Valid`
              (`GameplayStatics.PlaySound2D` NewSFX (`self.SFXVolume`) 1.0 0.0 null null)
              (`KismetSystemLibrary.PrintString` "SFX  재생됨")
              (if (not (== (`self.CurrentBGM`) NewBGM))
                (`/Engine/EditorBlueprintResources/StandardMacros.IsValid` _currentbgmcomponent
                  (:`Is Valid`
                    (`AudioComponent.FadeOut` _currentbgmcomponent _fadetime 0.0 "Linear"))
                  (:`Is Not Valid`
                    _))
                (`/Engine/EditorBlueprintResources/StandardMacros.IsValid` NewBGM
                  (:`Is Valid`
                    (bind _returnvalue (`GameplayStatics.SpawnSound2D` NewBGM 1.0 1.0 0.0 null))
                    (bind _output_get (set `self.CurrentBGMComponent` _returnvalue))
                    (`AudioComponent.FadeIn` _output_get _fadetime (`self.BGMVolume`) 0.0 "Linear")
                    (set `self.CurrentBGM` NewBGM)))))))))))

(fn `UserConstructionScript`)