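; BP_NPC is an NPC with a visible vision cone that follows its head and is clipped by obstacles.
; Each Tick fans downward-tilted Visibility line traces from VirtualHead and rebuilds VisionMesh as a procedural triangle fan from the hit or max-radius points.
; TurnHeadLeft and TurnHeadRight play timelines that sweep head yaw back and forth through summed clamped range mappings.
; NPCPath exposes the Path variable; no detection logic is present.
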(event `self.ReceiveTick`
  (params (DeltaSeconds :type "Float (single-precision)"))
  (bind _returnvalue (`SceneComponent.K2_GetComponentLocation` (`self.VirtualHead`)))
  (bind _returnvalue_2 (`SceneComponent.K2_GetComponentToWorld` (`self.VirtualHead`)))
  (`ProceduralMeshComponent.ClearAllMeshSections` (`self.VisionMesh`))
  (`KismetArrayLibrary.Array_Clear` (`self.Triangles`))
  (`KismetArrayLibrary.Array_Clear` (`self.Vertices`))
  (`KismetArrayLibrary.Array_Add` (`self.Vertices`))
  (for _index (range (+ (`KismetMathLibrary.FTrunc` (/ (`self.ViewAngle`) (`self.Resolution`))) 1))
    (bind _returnvalue_3 (+ _returnvalue (* (`KismetMathLibrary.GreaterGreater_VectorRotator` (`KismetMathLibrary.GetForwardVector` (`SceneComponent.K2_GetComponentRotation` (`self.VirtualHead`))) (`KismetMathLibrary.MakeRotator` 0.0 -10.0 (- (* _index (`self.Resolution`)) (/ (`self.ViewAngle`) 2.0)))) (`self.ViewRadius`))))
    (bind (_outhit _returnvalue_4) (`KismetSystemLibrary.LineTraceSingle` _returnvalue _returnvalue_3 "TraceTypeQuery1" false (`|MakeArray` self :!type "Actor Object Reference") "ForOneFrame"))
    (if _returnvalue_4
      (`KismetArrayLibrary.Array_Add` (`self.Vertices`) (`KismetMathLibrary.InverseTransformLocation` _returnvalue_2 (`.Location` (`GameplayStatics.BreakHitResult` _outhit))))
      (else
        (`KismetArrayLibrary.Array_Add` (`self.Vertices`) (`KismetMathLibrary.InverseTransformLocation` _returnvalue_2 _returnvalue_3)))))
  (for _index_2 (range 1 (+ (- (`KismetArrayLibrary.Array_Length` (`self.Vertices`)) 2) 1))
    (`KismetArrayLibrary.Array_Add` (`self.Triangles`))
    (`KismetArrayLibrary.Array_Add` (`self.Triangles`) (+ _index_2 1))
    (`KismetArrayLibrary.Array_Add` (`self.Triangles`) _index_2))
  (`ProceduralMeshComponent.CreateMeshSection_LinearColor` :`self` (`self.VisionMesh`) :`Vertices` (`self.Vertices`) :`Triangles` (`self.Triangles`))
  (`PrimitiveComponent.SetMaterial` (`self.VisionMesh`) 0 "/Game/NPC/M_VisionCone_Inst.M_VisionCone_Inst"))

(event `TurnHeadLeft`
  (bind (_direction _alpha) (`Timeline|H_Rotation_Timeline` :!via `PlayFromStart`)
    (:`Update`
      (`SceneComponent.K2_SetRelativeRotation` (`self.VirtualHead`) (`KismetMathLibrary.MakeRotator` 0.0 0.0 (+ (`KismetMathLibrary.MapRangeClamped` _alpha 0.0 1.0 0.0 -90.0) (`KismetMathLibrary.MapRangeClamped` _alpha 1.0 2.0 0.0 135.0) (`KismetMathLibrary.MapRangeClamped` _alpha 2.0 3.0 0.0 -225.0) (`KismetMathLibrary.MapRangeClamped` _alpha 3.0 4.0 0.0 180.0))) false false))))

(event `TurnHeadRight`
  (bind (_direction _alpha) (`Timeline|타임라인` :!via `PlayFromStart`)
    (:`Update`
      (`SceneComponent.K2_SetRelativeRotation` (`self.VirtualHead`) (`KismetMathLibrary.MakeRotator` 0.0 0.0 (+ (`KismetMathLibrary.MapRangeClamped` _alpha 0.0 1.0 0.0 90.0) (`KismetMathLibrary.MapRangeClamped` _alpha 1.0 2.0 0.0 -135.0) (`KismetMathLibrary.MapRangeClamped` _alpha 2.0 3.0 0.0 225.0) (`KismetMathLibrary.MapRangeClamped` _alpha 3.0 4.0 0.0 -180.0))) false false))))

(fn `NPC_Path`
  (returns (Path :type "/Game/Jamyip/BP_Way Object Reference"))
  (return (`self.Path`)))

(fn `UserConstructionScript`)