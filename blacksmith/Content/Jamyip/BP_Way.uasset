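; BP_Way is a waypoint path actor that hands out positions along a Spline component.
; A custom path event advances the PathPoint index and wraps it to zero after four points, a count hard-coded rather than read from the spline.
; The function 새함수 returns the world location of the spline point at the current index.
; BeginPlay, Tick, overlap and construction logic are empty, so it acts only when called.
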(event `path`
  (bind _output_get (set `self.Path Point` (+ (`self.Path Point`) 1)))
  (if (>= _output_get 4)
    (set `self.Path Point` 0)))

(fn `UserConstructionScript`)

(fn `새 함수`
  (returns (Location :type "Vector Structure"))
  (return (`SplineComponent.GetLocationAtSplinePoint` (`self.Spline`) (`self.Path Point`) "World")))