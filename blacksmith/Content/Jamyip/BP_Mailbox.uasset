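; BP_Mailbox is an interactable mailbox actor that starts the game mode's daily timer when the player presses F nearby.
; InteractRange overlaps with the third-person character toggle PlayerInRange and the InteractionUI widget component, which is labeled "우편함" (mailbox) and hidden at BeginPlay.
; The actor enables its own input for player 0, and F calls StartDailyTimer on BP_GameMode1 only while the player is in range.
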(event `self.interact range.OnComponentBeginOverlap`
  (params (OverlappedComponent :type "PrimitiveComponent Object Reference") (OtherActor :type "Actor Object Reference") (OtherComp :type "PrimitiveComponent Object Reference") (OtherBodyIndex :type Integer) (bFromSweep :type Boolean) (SweepResult :type "HitResult Structure (by ref)"))
  (cast `/Game/ThirdPerson/Blueprints/BP_ThirdPersonCharacter` OtherActor)
  (set `self.PlayerInRange` true)
  (`SceneComponent.SetVisibility` (`self.interactionUI`) true false))

(event `self.interact range.OnComponentEndOverlap`
  (params (OverlappedComponent :type "PrimitiveComponent Object Reference") (OtherActor :type "Actor Object Reference") (OtherComp :type "PrimitiveComponent Object Reference") (OtherBodyIndex :type Integer))
  (cast `/Game/ThirdPerson/Blueprints/BP_ThirdPersonCharacter` OtherActor)
  (set `self.PlayerInRange` false)
  (`SceneComponent.SetVisibility` (`self.interactionUI`) false false))

(event `Key|F`
  (params (Key :type "Key Structure"))
  (:`Pressed`
    (if (`self.PlayerInRange`)
      (bind _asbp_game_mode_1 (cast `/Game/jungbum/BP_GameMode1` (`GameplayStatics.GetGameMode`)))
      (`BlacksmithGameMode.StartDailyTimer` _asbp_game_mode_1))))

(event `self.ReceiveBeginPlay`
  (bind _interactionui (`self.interactionUI`))
  (bind _aswbp_button_ingame (cast `/Game/WBP/WBP_ButtonIngame` (`WidgetComponent.GetUserWidgetObject` _interactionui)))
  (set `/Game/WBP/WBP_ButtonIngame.AreaName` "우편함" _aswbp_button_ingame)
  (`SceneComponent.SetVisibility` _interactionui false false)
  (`self.EnableInput` (`GameplayStatics.GetPlayerController` 0)))

(fn `UserConstructionScript`)