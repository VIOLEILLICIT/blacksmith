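; BP_LeafRuneArea is an interaction zone actor that opens the leaf rune UI widget when the player presses F inside it.
; InteractionBox overlaps with any Character toggle IsInArea and enable or disable the actor's input for player controller 0, with debug prints.
; Pressing F while inside creates WBP_LeafRune, adds it to the viewport and shows the mouse cursor while setting Game Only input mode.
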(event `self.InteractionBox.OnComponentBeginOverlap`
  (params (OverlappedComponent :type "PrimitiveComponent Object Reference") (OtherActor :type "Actor Object Reference") (OtherComp :type "PrimitiveComponent Object Reference") (OtherBodyIndex :type Integer) (bFromSweep :type Boolean) (SweepResult :type "HitResult Structure (by ref)"))
  (cast `Character` OtherActor)
  (set `self.IsInArea` true)
  (`KismetSystemLibrary.PrintString` "Hello")
  (`self.EnableInput` (`GameplayStatics.GetPlayerController` 0)))

(event `self.InteractionBox.OnComponentEndOverlap`
  (params (OverlappedComponent :type "PrimitiveComponent Object Reference") (OtherActor :type "Actor Object Reference") (OtherComp :type "PrimitiveComponent Object Reference") (OtherBodyIndex :type Integer))
  (cast `Character` OtherActor)
  (set `self.IsInArea` false)
  (`KismetSystemLibrary.PrintString` "bye")
  (`self.DisableInput` (`GameplayStatics.GetPlayerController` 0)))

(event `Key|F`
  (params (Key :type "Key Structure"))
  (bind _returnvalue (`GameplayStatics.GetPlayerController` 0))
  (:`Pressed`
    (`KismetSystemLibrary.PrintString` "F")
    (if (`self.IsInArea`)
      (bind _returnvalue_2 (`|CreateWidget` "/Game/smith/leafRune/WBP_LeafRune.WBP_LeafRune_C"))
      (bind _output_get (set `self.LeafRuneWidgetRef` _returnvalue_2))
      (`UserWidget.AddToViewport` _output_get 0)
      (`UserWidget.AddToViewport` (`self.LeafRuneWidgetRef`) 0)
      (`WidgetBlueprintLibrary.SetInputMode_GameOnly` _returnvalue)
      (set `PlayerController.bShowMouseCursor` true _returnvalue))))

(fn `UserConstructionScript`)