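; BP_FireRuneArea is an interaction zone that opens the fire rune choice UI while a character stands inside.
; BeginPlay fits four hidden edge components to the Box scale and passes editable area, key and label text to the in-world WBP_ButtonIngame prompt.
; InteractionBox overlaps toggle the border, prompt and player input.
; IA_Interactive inside the zone creates WBP_FireRuneChoice and switches to UI-only input with a mouse cursor.
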(event `self.ReceiveBeginPlay`
  (bind _left (`self.Left`))
  (bind (_returnvalue_x _returnvalue_y) (`KismetMathLibrary.BreakVector` (`SceneComponent.K2_GetComponentScale` (`self.Box`))))
  (bind _returnvalue (* (- _returnvalue_y 1.0) 100.0))
  (bind _returnvalue_2 (* (- _returnvalue_x 1.0) 100.0))
  (`SceneComponent.SetVisibility` (`self.Widget`) false false) ; 윤예나
  (`SceneComponent.SetVisibility` _left false false)
  (`SceneComponent.SetVisibility` (`self.Right`) false false)
  (`SceneComponent.SetVisibility` (`self.Top`) false false)
  (`SceneComponent.SetVisibility` (`self.Bottom`) false false)
  (`SceneComponent.SetWorldScale3D` _left (`KismetMathLibrary.MakeVector` (- _returnvalue_x 0.8) 0.2 0.1))
  (`SceneComponent.SetWorldScale3D` (`self.Right`) (`KismetMathLibrary.MakeVector` (- _returnvalue_x 0.8) 0.2 0.1))
  (`SceneComponent.SetWorldScale3D` (`self.Top`) (`KismetMathLibrary.MakeVector` 0.2 (- _returnvalue_y 0.8) 0.1))
  (`SceneComponent.SetWorldScale3D` (`self.Bottom`) (`KismetMathLibrary.MakeVector` 0.2 (- _returnvalue_y 0.8) 0.1))
  (`SceneComponent.K2_SetRelativeLocation` (`self.Left`) (`KismetMathLibrary.MakeVector` 0.0 (/ _returnvalue -2.0)) false false)
  (`SceneComponent.K2_SetRelativeLocation` (`self.Right`) (`KismetMathLibrary.MakeVector` 0.0 (/ _returnvalue 2.0)) false false)
  (`SceneComponent.K2_SetRelativeLocation` (`self.Top`) (`KismetMathLibrary.MakeVector` (/ _returnvalue_2 2.0)) false false)
  (`SceneComponent.K2_SetRelativeLocation` (`self.Bottom`) (`KismetMathLibrary.MakeVector` (/ _returnvalue_2 -2.0)) false false)
  (bind _aswbp_button_ingame (cast `/Game/WBP/WBP_ButtonIngame` (`WidgetComponent.GetUserWidgetObject` (`self.Widget`))))
  (set `/Game/WBP/WBP_ButtonIngame.AreaName` (`self.AreaName Editable`) _aswbp_button_ingame)
  (set `/Game/WBP/WBP_ButtonIngame.KeyText` (`self.KeyText Editable`) _aswbp_button_ingame)
  (set `/Game/WBP/WBP_ButtonIngame.LabelText` (`self.LabelText Editable`) _aswbp_button_ingame)
  (set `/Game/WBP/WBP_ButtonIngame.bVisibleKeyBorderUI` (`self.bVisibleKeyBorder`) _aswbp_button_ingame))

(event `self.InteractionBox.OnComponentBeginOverlap`
  (params (OverlappedComponent :type "PrimitiveComponent Object Reference") (OtherActor :type "Actor Object Reference") (OtherComp :type "PrimitiveComponent Object Reference") (OtherBodyIndex :type Integer) (bFromSweep :type Boolean) (SweepResult :type "HitResult Structure (by ref)"))
  (cast `Character` OtherActor)
  (set `self.IsInArea` true)
  (`SceneComponent.SetVisibility` (`self.Right`) true false)
  (`SceneComponent.SetVisibility` (`self.Bottom`) true false)
  (`SceneComponent.SetVisibility` (`self.Top`) true false)
  (`SceneComponent.SetVisibility` (`self.Left`) true false)
  (`SceneComponent.SetVisibility` (`self.Widget`) true false)
  (`self.EnableInput` (`GameplayStatics.GetPlayerController` 0)))

(event `self.InteractionBox.OnComponentEndOverlap`
  (params (OverlappedComponent :type "PrimitiveComponent Object Reference") (OtherActor :type "Actor Object Reference") (OtherComp :type "PrimitiveComponent Object Reference") (OtherBodyIndex :type Integer))
  (cast `Character` OtherActor)
  (set `self.IsInArea` false)
  (`SceneComponent.SetVisibility` (`self.Right`) false false)
  (`SceneComponent.SetVisibility` (`self.Bottom`) false false)
  (`SceneComponent.SetVisibility` (`self.Top`) false false)
  (`SceneComponent.SetVisibility` (`self.Left`) false false)
  (`SceneComponent.SetVisibility` (`self.Widget`) false false)
  (`self.DisableInput` (`GameplayStatics.GetPlayerController` 0)))

(event `EnhancedInput|/Game/ThirdPerson/Input/Actions/IA_Interactive`
  (params (ActionValue :type "Float (double-precision)") (ElapsedSeconds :type "Float (double-precision)") (TriggeredSeconds :type "Float (double-precision)") (InputAction :type "InputAction Object Reference" :default "/Game/ThirdPerson/Input/Actions/IA_Interactive.IA_Interactive"))
  (bind _returnvalue (`GameplayStatics.GetPlayerController` 0))
  (:`Started`
    (if (`self.IsInArea`)
      (bind _returnvalue_2 (`|CreateWidget` "/Game/smith/fireRune/WBP_FireRuneChoice.WBP_FireRuneChoice_C"))
      (`UserWidget.AddToViewport` _returnvalue_2 0)
      (`WidgetBlueprintLibrary.SetInputMode_UIOnlyEx` _returnvalue _returnvalue_2)
      (set `PlayerController.bShowMouseCursor` true _returnvalue))))

(fn `UserConstructionScript`)